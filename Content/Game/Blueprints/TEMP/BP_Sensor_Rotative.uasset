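; Rotating sensor that sweeps its head back and forth through 180 degrees and detects the player staying inside its trigger zone.
; A timeline drives the sweep, with a FlipFlop alternating reverse and forward playback.
; Zone overlap starts a looping timer that fills the player's detection meter, calling DetectPlayer and OnDetected at the threshold.
; Leaving the zone resets the count, and the meter unless already detected.
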(event OnComponentBeginOverlap(TriggerDetectionZone)
  (params (OverlappedComponent :type Primitive%20Component%20Object%20Reference) (OtherActor :type Actor%20Object%20Reference) (OtherComp :type Primitive%20Component%20Object%20Reference) (OtherBodyIndex :type Integer) (bFromSweep :type Boolean) (SweepResult :type Hit%20Result%20Structure%20%28by%20ref%29))
  (if (Actor|ActorHasTag OtherActor "Player")
    (Variables|Default|SetIsPlayerInZone true)
    (bind _returnvalue (Utilities|Time|SetTimerbyEvent (delegate Custom|Count) 0.002 true))
    (Variables|Default|SetCountTimer _returnvalue)))

(event OnComponentEndOverlap(TriggerDetectionZone)
  (params (OverlappedComponent :type Primitive%20Component%20Object%20Reference) (OtherActor :type Actor%20Object%20Reference) (OtherComp :type Primitive%20Component%20Object%20Reference) (OtherBodyIndex :type Integer))
  (bind _playerref (Variables|Default|GetPlayerRef))
  (bind _detectionmeterref (Variables|/Game/Game/Blueprints/Characters/Player/BP_Player.BP_Player_C|GetDetectionMeterRef _playerref))
  (if (Actor|ActorHasTag OtherActor "Player")
    (Variables|Default|SetIsPlayerInZone false)
    (Utilities|Time|ClearandInvalidateTimerbyHandle (Variables|Default|GetCountTimer))
    (Variables|Default|SetTimeUnderZone 0.0)
    (if (not (Variables|/Game/Game/Widget/WB_DetectionMeter.WB_DetectionMeter_C|GetHasBeenDetected _detectionmeterref))
      (Progress|SetPercent (Variables|/Game/Game/Widget/WB_DetectionMeter.WB_DetectionMeter_C|GetDetectionBar _detectionmeterref) 0.0))))

(event Custom|Count
  (Variables|Default|SetTimeUnderZone (+ (Variables|Default|GetTimeUnderZone) 0.005))
  (CallFunction|UpdateDetectionMeter)
  (if (>= (Variables|Default|GetTimeUnderZone) (Variables|Default|GetPlayerDetectionTimer))
    (CallFunction|DetectPlayer (stale OnComponentBeginOverlap(TriggerDetectionZone) OtherActor))
    (Utilities|Time|ClearandInvalidateTimerbyHandle (Variables|Default|GetCountTimer))
    (Default|OnDetected (Variables|/Game/Game/Blueprints/Characters/Player/BP_Player.BP_Player_C|GetDetectionMeterRef (Variables|Default|GetPlayerRef)))))

(event Custom|UpdateDetectionMeter
  (bind _playerref (Variables|Default|GetPlayerRef))
  (bind _detectionmeterref (Variables|/Game/Game/Blueprints/Characters/Player/BP_Player.BP_Player_C|GetDetectionMeterRef _playerref))
  (if (not (Variables|/Game/Game/Widget/WB_DetectionMeter.WB_DetectionMeter_C|GetHasBeenDetected _detectionmeterref))
    (Progress|SetPercent (Variables|/Game/Game/Widget/WB_DetectionMeter.WB_DetectionMeter_C|GetDetectionBar _detectionmeterref) (/ (Variables|Default|GetTimeUnderZone) (Variables|Default|GetPlayerDetectionTimer)))))

(event EventBeginPlay
  (Utilities|FlowControl|Sequence
    (:then_0
      (bind _rotation (Timeline|TL_Motion Play)
        (:Update
          (Transformation|SetRelativeRotation (Variables|Default|GetHead) (Math|Rotator|Lerp(Rotator) "0, 0, 0" "0.000000,180.000000,0.000000" _rotation) false false))
        (:Finished
          (Utilities|FlowControl|FlipFlop
            (:A
              (Timeline|TL_Motion ReverseFromEnd))
            (:B
              (Timeline|TL_Motion PlayFromStart))))))
    (:then_1
      (bind _asbp_player (Utilities|Casting|CastToBP_Player (Game|GetPlayerCharacter 0)))
      (Variables|Default|SetPlayerRef _asbp_player))))

(fn ConstructionScript
  (|CallParentFunction))