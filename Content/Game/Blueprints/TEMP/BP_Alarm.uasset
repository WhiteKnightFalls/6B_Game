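; BP_Alarm is an alarm actor that sounds a siren and alerts guards.
; StartAlarm spawns the siren at its location and calls AlertNearbyGuards, while StopAlarm fades the sound out, both gated by an active flag.
; Despite its name, AlertNearbyGuards has no distance check: it gets every BP_Guard and sets HasSeenPlayer on each BP_AI_Guard controller's blackboard, which stopping never clears.
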(event Custom|StartAlarm
  (if (not (Variables|Default|GetIsAlarmActive))
    (bind _returnvalue (Audio|SpawnSoundatLocation "/Game/Game/Audio/SFX/emergency_siren.emergency_siren" (Transformation|GetActorLocation) "0, 0, 0" 1.0 1.0 0.0 0 0))
    (Variables|Default|SetAlarmSound _returnvalue)
    (Variables|Default|SetIsAlarmActive true)
    (CallFunction|AlertNearbyGuards)))

(event Custom|StopAlarm
  (if (Variables|Default|GetIsAlarmActive)
    (Audio|Components|Audio|FadeOut (Variables|Default|GetAlarmSound) 1.0 0.0 "Linear" :!class /Script/Engine.AudioComponent)
    (Variables|Default|SetIsAlarmActive false)))

(event Custom|AlertNearbyGuards
  (bind _outactors (Actor|GetAllActorsOfClass "/Game/Game/Blueprints/Characters/NPC/BP_Guard.BP_Guard_C"))
  (for _array_element _outactors
    (bind _asbp_ai_guard (Utilities|Casting|CastToBP_AI_Guard (AI|GetAIController _array_element)))
    (AI|Components|Blackboard|SetValueasBool (AI|GetBlackboard _asbp_ai_guard) (Utilities|Name|MakeLiteralName "HasSeenPlayer") true)))

(event EventBeginPlay)

(fn ConstructionScript)