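; BP_Guard is an NPC guard character that can run and catch the player.
; Run sets the movement component's walk speed, while Catch plays a montage guarded by an IsCatching flag.
; A montage notify fires a debug-drawn forward sphere trace against Pawns.
; The first hit on a Player-tagged actor tells GM_BaseGameMode to show the captured screen, limited by a DoOnce.
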(event EventBeginPlay)

(event Collision|EventActorBeginOverlap
  (params (OtherActor :type Actor%20Object%20Reference)))

(event EventTick
  (params (DeltaSeconds :type Float%20%28single-precision%29)))

(event EventRun
  (Variables|/Script/Engine.CharacterMovementComponent|SetMaxWalkSpeed (Variables|Character|GetCharacterMovement) (Variables|Default|GetMaxWalkSpeed)))

(event EventCatch
  (bind _returnvalue (Transformation|GetActorLocation))
  (if (not (Variables|Default|GetIsCatching))
    (Animation|Montage|PlayMontage (Variables|Character|GetMesh) (Variables|Default|GetCatchMontage) 1.0 0.0 "None" false
      (:then
        (Variables|Default|SetIsCatching true))
      (:OnCompleted
        (Variables|Default|SetIsCatching false))
      (:OnNotifyBegin
        (bind (_outhit _returnvalue_2) (Collision|SphereTraceForObjects _returnvalue (+ _returnvalue (* (Transformation|GetActorForwardVector) (Variables|Default|GetCatchTraceLength))) 25.0 (Utilities|Array|MakeArray "ObjectTypeQuery3") false 0 "ForDuration"))
        (if _returnvalue_2
          (if (Actor|ActorHasTag (.HitActor (Collision|BreakHitResult _outhit)) "Player")
            (Utilities|FlowControl|DoOnce false
              (:Completed
                (bind _asgm_base_game_mode (Utilities|Casting|CastToGM_BaseGameMode (Game|GetGameMode)))
                (Default|CapturedScreen _asgm_base_game_mode)))))))))

(fn ConstructionScript)