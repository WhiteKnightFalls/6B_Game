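; Sensor actor that raises an alarm the first time it is told it has detected an actor tagged Player.
; DetectPlayer latches HasDetected, plays an attenuated sound at the sensor, starts the alarm through AlarmRef and drives the point light's intensity with a timeline.
; AlarmRef is not assigned in these graphs, as the BP_Alarm lookup is left unconnected.
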(event Custom|DetectPlayer
  (params (ActorDetected :type Actor%20Object%20Reference))
  (if (and (Actor|ActorHasTag ActorDetected "Player") (not (Variables|Default|GetHasDetected)))
    (Variables|Default|SetHasDetected true)
    (Audio|PlaySoundatLocation 0 (Transformation|GetActorLocation) "0, 0, 0" 1.0 1.0 0.0 "/Game/Game/Audio/Sound_Attenuation/SA_Sensor.SA_Sensor" 0 0 0)
    (Default|StartAlarm (Variables|Default|GetAlarmRef))
    (bind _intensity (Timeline|TL_PointLight Play)
      (:Update
        (Rendering|Components|Light|SetIntensity (Variables|Default|GetPointLight) (Math|Float|Lerp 0.0 1e+02 _intensity))))))

(fn ConstructionScript)