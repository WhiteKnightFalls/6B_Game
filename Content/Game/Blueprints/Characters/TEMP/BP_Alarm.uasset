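; Temporary alarm actor that plays a sound at its location, starting automatically three seconds after BeginPlay.
; StartAlarm spawns an editor-style placeholder sound (Dockable_Window_Close) and stores the audio component, while StopAlarm fades it out over one second.
; An IsAlarmActive flag guards both events against repeat triggering, and nothing in this Blueprint calls StopAlarm.
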(event Custom|StartAlarm
  (if (not (Variables|Default|GetIsAlarmActive))
    (bind _returnvalue (Audio|SpawnSoundatLocation "/Engine/VREditor/Sounds/UI/Dockable_Window_Close.Dockable_Window_Close" (Transformation|GetActorLocation) "0, 0, 0" 1.0 1.0 0.0 0 0))
    (Variables|Default|SetAlarmSound _returnvalue)
    (Variables|Default|SetIsAlarmActive true)))

(event Custom|StopAlarm
  (if (Variables|Default|GetIsAlarmActive)
    (Audio|Components|Audio|FadeOut (Variables|Default|GetAlarmSound) 1.0 0.0 "Linear" :!class /Script/Engine.AudioComponent)
    (Variables|Default|SetIsAlarmActive false)))

(event EventBeginPlay
  (Utilities|FlowControl|Delay 3.0)
  (CallFunction|StartAlarm))

(fn ConstructionScript)