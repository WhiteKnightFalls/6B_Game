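; Checkpoint actor that registers itself as the player's current checkpoint when BP_Player overlaps its sphere.
; The overlap spawns stylized smoke above the actor and destroys that effect after a five-second delay.
; GetRespawnLocRot supplies the respawn point's rotation and slightly offset location.
; SaveCheckpoint can write a location to a save slot, but its only graph call never runs, and LoadCheckpoint is empty.
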(event OnComponentBeginOverlap(Sphere)
  (params (OverlappedComponent :type Primitive%20Component%20Object%20Reference) (OtherActor :type Actor%20Object%20Reference) (OtherComp :type Primitive%20Component%20Object%20Reference) (OtherBodyIndex :type Integer) (bFromSweep :type Boolean) (SweepResult :type Hit%20Result%20Structure%20%28by%20ref%29))
  (bind _asbp_player (Utilities|Casting|CastToBP_Player OtherActor))
  (Variables|/Game/Game/A_Blueprints/Player/BP_Player.BP_Player_C|SetMyCheckpoint _asbp_player self)
  (bind _returnvalue (Niagara|SpawnSystematLocation "/Game/Game/F_VFX/Niagara/Systems/NS_StylizedSmoke.NS_StylizedSmoke" (+ (Transformation|GetActorLocation) "0.000000,0.000000,150.000000")))
  (bind _output_get (Variables|Default|SetVFX _returnvalue))
  (Utilities|FlowControl|Delay 5.0)
  (Components|DestroyComponent _output_get))

(event EventBeginPlay)

(event Collision|EventActorBeginOverlap
  (params (OtherActor :type Actor%20Object%20Reference)))

(event EventTick
  (params (DeltaSeconds :type Float%20%28single-precision%29)))

(fn ConstructionScript)

(fn SaveCheckpoint
  (params (CheckpointLocation :type Vector))
  (bind _returnvalue (SaveGame|CreateSaveGameObject "/Game/Game/H_Systems/BP_SaveGame.BP_SaveGame_C"))
  (Variables|/Game/Game/H_Systems/BP_SaveGame.BP_SaveGame_C|SetLastCheckpointLocation _returnvalue CheckpointLocation)
  (bind _returnvalue_2 (SaveGame|SaveGametoSlot _returnvalue "checkpoint"))
  (if _returnvalue_2
    (Niagara|SpawnSystematLocation "/Game/Game/F_VFX/Niagara/Systems/NS_StylizedSmoke.NS_StylizedSmoke" (+ (Transformation|GetActorLocation) "0.000000,0.000000,150.000000"))))

(fn LoadCheckpoint)

(fn GetRespawnLocRot
  (bind _checkpointrespawnpoint (Variables|Default|GetCheckpointRespawnPoint))
  (return (- (Transformation|GetWorldLocation _checkpointrespawnpoint) "-20.000000,-20.000000,0.000000") (Transformation|GetWorldRotation _checkpointrespawnpoint)))