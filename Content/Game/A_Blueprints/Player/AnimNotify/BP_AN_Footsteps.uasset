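; Anim notify that plays a surface-dependent footstep sound for the player's left or right foot.
; It traces down through the ball socket of the foot chosen by IsRightFoot, ignoring the owner, with debug drawing left on.
; On a hit, the physical surface selects dirt, wood or concrete audio, falling back to dirt.
; The sound plays attenuated at the impact location, at a volume picked by SFXVolumeIndex.
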(fn ReceivedNotify
  (params (MeshComp :type Skeletal%20Mesh%20Component%20Object%20Reference) (Animation :type Anim%20Sequence%20Base%20Object%20Reference) (EventReference :type Anim%20Notify%20Event%20Reference%20Structure%20%28by%20ref%29))
  (bind _isrightfoot (Variables|Default|GetIsRightFoot))
  (bind _returnvalue (select _isrightfoot "ball_r" "ball_l"))
  (bind _returnvalue_2 (Transformation|GetSocketLocation MeshComp _returnvalue))
  (bind (_outhit _returnvalue_3) (Collision|LineTraceByChannel (+ _returnvalue_2 "0.000000,0.000000,25.000000") (- _returnvalue_2 "0.000000,0.000000,90.000000") "TraceTypeQuery1" false (Utilities|Array|MakeArray (Components|GetOwner MeshComp)) "ForDuration" true "(R=1.000000,G=0.000000,B=0.000000,A=1.000000)" "(R=0.000000,G=1.000000,B=0.000000,A=1.000000)" 2.0))
  (if _returnvalue_3
    (Audio|PlaySoundatLocation (Utilities|Select :Index (Variables|/Script/PhysicsCore.PhysicalMaterial|GetSurfaceType (.PhysMat (Collision|BreakHitResult _outhit))) :SurfaceType_Default "/Game/Game/D_Audio/SFX/SoundCues/SC_SFX_Footsteps_Dirt.SC_SFX_Footsteps_Dirt" :SurfaceType1 "/Game/Game/D_Audio/SFX/SoundCues/SC_SFX_Footsteps_Dirt.SC_SFX_Footsteps_Dirt" :SurfaceType2 "/Game/Game/D_Audio/SFX/SoundCues/SC_SFX_Footsteps_Wood.SC_SFX_Footsteps_Wood" :SurfaceType3 "/Game/Game/D_Audio/SFX/SoundCues/SC_SFX_Footsteps_Concrete.SC_SFX_Footsteps_Concrete") (.Location (Collision|BreakHitResult _outhit)) "0, 0, 0" (Utilities|Select :Index (Variables|Default|GetSFXVolumeIndex) :Option%200 1.0 :Option%201 0.75 :Option%202 0.5 :Option%203 0.25) 1.0 0.0 "/Game/Game/D_Audio/SoundAttenuation/SA_Footsteps.SA_Footsteps" 0 0 0)))