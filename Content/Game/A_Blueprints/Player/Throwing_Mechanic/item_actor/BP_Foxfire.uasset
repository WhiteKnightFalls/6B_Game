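; BP_Foxfire is a throwable foxfire item actor that makes a noise AI hearing can detect where it lands.
; Hits are ignored until one second after BeginPlay, then a DoOnce plays the impact sound, reports the noise and sets ENDSHOW.
; TheItem stops simulating physics shortly after impact, and the actor destroys itself a few seconds later.
; Unconnected leftover nodes include a glass-bottle fracture spawn that never runs.
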(event EventBeginPlay
  ;[1 1 1] Comment
  (|CallParentFunction)
  (Utilities|FlowControl|Delay 1.0)
  (Variables|Default|Setstart%20action true))

(event Collision|EventHit
  (params (MyComp :type Primitive%20Component%20Object%20Reference) (Other :type Actor%20Object%20Reference) (OtherComp :type Primitive%20Component%20Object%20Reference) (bSelfMoved :type Boolean) (HitLocation :type Vector :default "0, 0, 0") (HitNormal :type Vector :default "0, 0, 0") (NormalImpulse :type Vector :default "0, 0, 0") (Hit :type Hit%20Result%20Structure%20%28by%20ref%29))
  (if (Variables|Default|Getstart%20action)
    (Utilities|FlowControl|DoOnce false
      (:Completed
        (Audio|PlaySoundatLocation "/Game/Game/D_Audio/SFX/Player/SFX_Foxfire_Impact.SFX_Foxfire_Impact" HitLocation "0, 0, 0" 1.0 1.0 0.0 "/Game/Game/D_Audio/SoundAttenuation/SA_FoxFire.SA_FoxFire" 0 0 0)
        (Class|AISenseHearing|ReportNoiseEvent HitLocation 1.2 self 0.0 "None")
        (Variables|Default|SetEND%20SHOW true)
        (Utilities|FlowControl|Delay 0.2)
        (Physics|SetSimulatePhysics (Variables|Default|Getthe_item) false)
        (Utilities|FlowControl|Delay 4.0)
        (Actor|DestroyActor)))))

(fn ConstructionScript
  (|CallParentFunction))