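; Player ability cooldown component that tracks a countdown and exposes whether it is active and its remaining fraction.
; StartCooldown resets CurrentCooldown to Cooldown, then Tick lowers it to zero with FInterpToConstant at a fixed 1.5 units per second, so faster than real seconds.
; Tick also prints the remaining value while active, and CustomEvent is an unfinished stub that checks the active state without acting.
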(event Custom|StartCooldown
  (Variables|Default|SetcurrentCooldown (Variables|Default|Getcooldown)))

(event Custom|CustomEvent
  (bind _isoncooldown (CallFunction|IsCooldownActive))
  (if _isoncooldown
    _))

(event EventTick
  (params (DeltaSeconds :type Float%20%28single-precision%29))
  (bind _isoncooldown (CallFunction|IsCooldownActive))
  (if _isoncooldown
    (Variables|Default|SetcurrentCooldown (Math|Interpolation|FInterptoConstant (Variables|Default|GetcurrentCooldown) 0.0 (Utilities|Time|GetWorldDeltaSeconds) 1.5))
    (Development|PrintString (Utilities|String|ToString(Float) (Variables|Default|GetcurrentCooldown)))))

(fn IsCooldownActive
  (return (> (Variables|Default|GetcurrentCooldown) 0.0)))

(fn GetRelativeCooldown
  (return (/ (Variables|Default|GetcurrentCooldown) (Variables|Default|Getcooldown))))