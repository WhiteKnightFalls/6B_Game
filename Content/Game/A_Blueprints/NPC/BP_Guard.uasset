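; Guard NPC that patrols a path and shows a detection meter, with its AI handled by the BP_AI_Guard controller.
; On BeginPlay it caches controller and player, then after a short delay tells the controller to patrol with timed stops and head-gesture montages.
; Hits are reported to AI perception as touch events.
; Each tick it turns the meter toward the player's camera and copies the controller's hearing flag.
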(event EventBeginPlay
  ;[1 0.09198 0.4769 1 24] Setup
  (Utilities|FlowControl|Sequence
    (:then_0
      (bind _asbp_ai_guard (Utilities|Casting|CastToBP_AI_Guard (Pawn|GetController)))
      (Variables|Default|SetAIGuardRef _asbp_ai_guard))
    (:then_1
      (Utilities|FlowControl|Delay 0.2)
      (Default|MoveinPath (Variables|Default|GetAIGuardRef) (Variables|Default|GetGuardPathingRef) 1 (Utilities|Map|MakeMap 2 2.0 4 3.0) (Utilities|Array|MakeArray "/Game/Game/A_Blueprints/NPC/animation/MONTAGE/MN_ThoughtfulHeadNod_Montage.MN_ThoughtfulHeadNod_Montage" "/Game/Game/A_Blueprints/NPC/animation/MONTAGE/MN_ThoughtfulHeadShake_Montage.MN_ThoughtfulHeadShake_Montage")))
    (:then_2
      (bind _asbp_player (Utilities|Casting|CastToBP_Player (Game|GetPlayerCharacter 0)))
      (Variables|Default|SetPlayerRef _asbp_player))))

(event Collision|EventHit
  (params (MyComp :type Primitive%20Component%20Object%20Reference) (Other :type Actor%20Object%20Reference) (OtherComp :type Primitive%20Component%20Object%20Reference) (bSelfMoved :type Boolean) (HitLocation :type Vector :default "0, 0, 0") (HitNormal :type Vector :default "0, 0, 0") (NormalImpulse :type Vector :default "0, 0, 0") (Hit :type Hit%20Result%20Structure%20%28by%20ref%29))
  ;[0.522 1 0.5805 1 24] report touch to ai
  (Class|AISenseTouch|ReportTouchEvent self Other HitLocation))

(event EventTick
  (params (DeltaSeconds :type Float%20%28single-precision%29))
  ;[0.3288 0.9618 1 1 24] facing the widget to player camera
  (Utilities|FlowControl|Sequence
    (:then_0
      (Transformation|SetWorldRotation (Variables|Default|GetDetectionMeter) (Math|Rotator|FindLookatRotation (Transformation|GetWorldLocation (Variables|Default|GetDetectionMeter)) (Transformation|GetWorldLocation (Variables|/Game/Game/A_Blueprints/Player/BP_Player.BP_Player_C|GetCamera (Variables|Default|GetPlayerRef)))) false false))
    (:then_1
      (Variables|Default|SetIs%20Hearing%20Sound (Variables|/Game/Game/A_Blueprints/NPC/BP_AI_Guard.BP_AI_Guard_C|GetIsHearingSound (Variables|Default|GetAIGuardRef))))))

(fn ConstructionScript)