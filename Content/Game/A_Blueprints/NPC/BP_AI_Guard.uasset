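; Guard AI controller that patrols spline paths with timed animation stops, investigates sounds, and chases and damages the player.
; AI Perception sight, touch and hearing set state flags and detection levels that Tick evaluates.
; A widget meter on the guard shows detection, also influenced by a dot-product and sphere-trace check for a player behind it.
; DoOnce gates control chase transitions, and a lose-sight timer plus distance check returns the guard to patrol.
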(event OnTargetPerceptionUpdated(AIPerception)
  (params (Actor :type Actor%20Object%20Reference) (Stimulus :type AI%20Stimulus%20Structure))
  ;[0 0.8398 1 1 24] AI Perception
  (CallFunction|AIPerceptionSight Actor Stimulus)
  (CallFunction|AIPerceptionTouch Actor Stimulus)
  (CallFunction|AIPerceptionHearing Actor Stimulus))

(event Custom|DetectionAction
  (bind _detectionmeterwidget (Variables|References|GetDetectionMeterWidget))
  (bind _detectionmeterwidget_2 (Variables|References|GetDetectionMeterWidget))
  (bind _detectionmeterwidget_3 (Variables|References|GetDetectionMeterWidget))
  ;[0.8745 0.7298 1 1 24] increases/decreases Detection Meter
  (if (== (Variables|Default|GetCurrentTargetDetection) 1.0)
    (Utilities|FlowControl|DoOnce false
      (:Completed
        (CallFunction|GotoPlayer)))
    (elif (Variables|AiAction|GetStartDetectionMeter)
      (bind _output_get (Variables|Default|SetCurrentTargetDetection (Math|Interpolation|FInterptoConstant (Variables|Default|GetCurrentTargetDetection) 1.0 (Utilities|Time|GetWorldDeltaSeconds) (Variables|Default|GetTimerRaiseDetection))))
      (Utilities|IsValid _detectionmeterwidget_3
        (:Is%20Valid
          (Default|UpdatePercent _detectionmeterwidget_3 _output_get)
          (Widget|SetVisibility (Variables|References|GetDetectionMeterWidget) "Visible" :!label _label)))
      (elif (not (and (Variables|AiAction|GetHasSeenPlayer) (Variables|AiAction|GetIsChasingPlayer)))
        (if (!= (Variables|Default|GetCurrentTargetDetection) 0.0)
          (bind _output_get_2 (Variables|Default|SetCurrentTargetDetection (Math|Interpolation|FInterptoConstant (Variables|Default|GetCurrentTargetDetection) 0.0 (Utilities|Time|GetWorldDeltaSeconds) (Variables|Default|GetTimerDropDetection))))
          (Utilities|IsValid _detectionmeterwidget_2
            (:Is%20Valid
              (Default|UpdatePercent _detectionmeterwidget_2 _output_get_2)
              (goto _label)))
          (else
            (Utilities|IsValid _detectionmeterwidget
              (:Is%20Valid
                (Widget|SetVisibility _detectionmeterwidget "Hidden")))))))))

(event Custom|move%20in%20path
  (params (Pathing :type Array%20of%20BP%20Guard%20Pathing%20Object%20References) (PathingNumber :type Integer) (StoptimerAtPath :type Map%20of%20Integers%20to%20Reals) (StopAnimation :type Array%20of%20Anim%20Montage%20Object%20References))
  ;[1 0.86 0.3047 0.688 24] Whole Guard Pathing Logic
  ;;[0.5906 0.7083 0.5152 0.844] move in path event
  (bind _output_get (Variables|aipath|SetALL%20Paths Pathing))
  (bind _output_get_2 (Variables|AiPath|SetPath%20Number (- PathingNumber 1)))
  (bind _output_get_3 (Variables|AiPath|SetStop%20Point StoptimerAtPath))
  (bind _output_get_4 (Variables|AiPath|SetStop%20Animation StopAnimation))
  (bind _output_get_5 (Variables|References|SetGuardPathingRef (Utilities|Array|Get(acopy) _output_get _output_get_2)))
  (CallFunction|LogicMoveinPath _output_get_5 _output_get_2 _output_get_3 _output_get_4))

(event Custom|ResetDetctionMeter
  (bind _detectionmeterwidget (Variables|References|GetDetectionMeterWidget))
  ;[0.5178 0.6816 0.8385 0.839] Checks if the Player is behind Guard
  (Utilities|FlowControl|Sequence
    (:then_0
      (Utilities|FlowControl|DoOnce false) ; enters at Reset
    )
    (:then_1
      (Variables|Default|SetCurrentTargetDetection 0.0)
      (Variables|AiAction|SetStartDetectionMeter false)
      (Utilities|IsValid _detectionmeterwidget
        (:Is%20Valid
          (Widget|SetVisibility _detectionmeterwidget "Hidden"))))))

(event Custom|SeePlayerForTheFirstTime
  (params (active :type Boolean))
  ;[1 1 1] logic see player in the first time
  (if active
    (Utilities|FlowControl|Delay 0.15)
    (Components|Movement|StopMovementImmediately (Variables|References|GetGuardMovementCompRef))
    (Variables|Default|SetCurrentTargetDetection (Math|Float|Clamp(Float) (+ (Variables|Default|GetCurrentTargetDetection) 0.35) 0.0 0.9))
    (Variables|AiAction|SetStartDetectionMeter true)
    (else
      (CallFunction|ReturntoPathing)
      (Variables|AiAction|SetStartDetectionMeter false))))

(event Custom|MoveAIToSoundLocation
  (params (Destination :type Vector))
  ;[1 0.1739 0.1849 1 24] Sound Perception Logic
  (Utilities|FlowControl|DoOnce false :!label _label
    (:Completed
      (Variables|aiaction|SetToSoundLocation true)
      (AI|AIMoveTo (Variables|References|GetCharacterRef) Destination 0 5e+01 false
        (:then
          (Animation|StopAnimMontage (Variables|References|GetCharacterRef) (Variables|AiPath|Getthe%20stop%20animation)))
        (:OnSuccess
          (Variables|AiAction|SetIsHearingSound true)
          (Utilities|FlowControl|Delay (Variables|Default|GetTimerSearchingSound))
          (CallFunction|ReturntoPathing)
          (Variables|AiAction|SetIsHearingSound false)
          (Variables|aiaction|SetToSoundLocation false)
          (goto _label Reset))))))

(event Custom|LastTimeHasSeenPlayer
  ;[1 1 1] Timer after losing Player
  (if (Variables|AiAction|GetHasSeenPlayer)
    (Variables|Default|SetTimerLosingPlayer 3.5)
    (elif (Variables|AiAction|GetIsChasingPlayer)
      (Variables|Default|SetTimerLosingPlayer (Math|Interpolation|FInterptoConstant (Variables|Default|GetTimerLosingPlayer) 0.0 (Utilities|Time|GetWorldDeltaSeconds) 3.5)))))

(event Custom|CheckDistance
  ;[1 1 1] Check Distance
  (if (> (CallFunction|CalculateDistance) 1e+03)
    (Variables|AiAction|SetIsPlayerClose false)
    (else
      (Variables|AiAction|SetIsPlayerClose true))))

(event Custom|CheckBack
  (bind _characterref (Variables|References|GetCharacterRef))
  ;[0.5178 0.6816 0.8385 0.839] Checks if the Player is behind Guard
  (if (not (Variables|AiAction|GetIsChasingPlayer))
    (if (< (CallFunction|CalculateDistance) 1e+03)
      (bind _output_get (Variables|Default|SetAngleSee (Math|Vector|DotProduct (Math|Vector|GetForwardVector (Transformation|GetActorRotation _characterref)) (- (Transformation|GetActorLocation (Variables|References|GetPlayerRef)) (Transformation|GetActorLocation _characterref)))))
      (if (<= _output_get -1.0)
        (bind (_outhit _returnvalue) (Collision|SphereTraceForObjects (Transformation|GetSocketLocation (Variables|/Script/Engine.Character|GetMesh (Variables|References|GetCharacterRef)) "head") (+ (Transformation|GetActorLocation (Variables|References|GetPlayerRef)) "0.000000,0.000000,35.000000") 1e+01 (Utilities|Array|MakeArray "ObjectTypeQuery1" "ObjectTypeQuery2" "ObjectTypeQuery3") false (Utilities|Array|MakeArray (Variables|References|GetCharacterRef)) "None"))
        (if _returnvalue
          (if (Utilities|Enum|Equal(Enum) (Collision|GetCollisionObjectType (.HitComponent (Collision|BreakHitResult _outhit))) "ECC_Pawn")
            (bind _asbp_player (Utilities|Casting|CastToBP_Player (.HitActor (Collision|BreakHitResult _outhit))))
            (if (AI|Components|NavMovement|IsCrouching (Variables|/Script/Engine.Character|GetCharacterMovement _asbp_player))
              (Utilities|FlowControl|DoOnce false :!label _label
                (:Completed
                  (Variables|AiAction|SetStartDetectionMeter false)
                  (goto _label_2 Reset)))
              (else
                (Utilities|FlowControl|DoOnce false :!label _label_2
                  (:Completed
                    (Variables|AiAction|SetStartDetectionMeter true)
                    (goto _label Reset)))))
            (else
              (Variables|AiAction|SetStartDetectionMeter false)))))
      (else
        (CallFunction|ResetDetctionMeter)))))

(event Custom|ChasingPlayer
  ;[0.008364 0.5729 0 1 24] Chasing Player Logic
  (Utilities|FlowControl|Sequence
    (:then_0
      (if (and (Variables|AiAction|GetHasSeenPlayer) (not (Variables|AiAction|GetIsChasingPlayer)))
        (Utilities|FlowControl|DoOnce false :!label _label
          (:Completed
            (CallFunction|SeePlayerfortheFirstTime true)
            (Utilities|FlowControl|Delay (Variables|Default|GetTimeToCheck))
            (if (Variables|AiAction|GetHasSeenPlayer)
              (Variables|Default|SetCurrentTargetDetection 0.99)
              (CallFunction|GotoPlayer :!label _label_2)
              (else
                (CallFunction|SeePlayerfortheFirstTime false)
                (goto _label Reset)))))))
    (:then_1
      (if (Variables|AiAction|GetIsTouchingPlayer)
        (goto _label_2)))
    (:then_2
      (if (not (Variables|AiAction|GetHasSeenPlayer))
        (CallFunction|StopChasingPlayer)))))

(event Custom|GoToPlayer
  ;[1 0.2536 0.1944 1 24] when ai can/can't catch the player logic
  (Utilities|FlowControl|DoOnce false
    (:Completed
      (Utilities|FlowControl|Delay 0.15)
      (Animation|StopAnimMontage (Variables|References|GetCharacterRef) (Variables|AiPath|Getthe%20stop%20animation))
      (Components|Movement|StopMovementImmediately (Variables|References|GetGuardMovementCompRef))
      (AI|AIMoveTo (Variables|References|GetCharacterRef) "0, 0, 0" (Variables|References|GetPlayerRef) 1e+01 false :!label _label
        (:then
          (Utilities|FlowControl|DoOnce false
            (:Completed
              (Variables|AiAction|SetIsChasingPlayer true)
              (Variables|/Script/Engine.CharacterMovementComponent|SetMaxWalkSpeed (Variables|References|GetGuardMovementCompRef) (Variables|Default|GetChasingSpeed))
              (Variables|AiAction|SetStartDetectionMeter true)
              (Variables|AiAction|SetIsHearingSound false)
              (Variables|aiaction|SetToSoundLocation false))))
        (:OnSuccess
          (Game|Damage|ApplyDamage (Variables|References|GetPlayerRef) 1e+02 0 0)
          (if (Variables|AiAction|GetIsChasingPlayer)
            (Utilities|FlowControl|Delay 1.0)
            (if (Variables|AiAction|GetIsChasingPlayer)
              (goto _label))))
        (:OnFail
          (if (Variables|AiAction|GetIsChasingPlayer)
            (Utilities|FlowControl|Delay 0.2)
            (if (Variables|AiAction|GetIsChasingPlayer)
              (goto _label))))))))

(event Custom|StopChasingPlayer
  ;[0.002964 1 0.03901 1 24] Stop Chasing Player Logic
  (if (Math|Boolean|ANDBoolean (Variables|AiAction|GetIsChasingPlayer) (== (Variables|Default|GetTimerLosingPlayer) 0.0) (> (CallFunction|CalculateDistance) 4.5e+02))
    (Utilities|FlowControl|DoOnce false
      (:Completed
        (Components|Movement|StopMovementImmediately (Variables|References|GetGuardMovementCompRef))
        (Variables|/Script/Engine.CharacterMovementComponent|SetMaxWalkSpeed (Variables|References|GetGuardMovementCompRef) (Variables|Default|GetDefaultWalkSpeed))
        (Variables|AiAction|SetIsChasingPlayer false)
        (CallFunction|ReturntoPathing)
        (CallFunction|ResetDoOnce)
        (CallFunction|ResetDetctionMeter)
        (Variables|aiaction|SetToSoundLocation false)))))

(event Custom|ResetDoOnce
  (Utilities|FlowControl|Sequence
    (:then_0
      (Utilities|FlowControl|Sequence
        (:then_0
          ;[1 0.2536 0.1944 1 24] when ai can/can't catch the player logic
          ;;[1 1 1] delay to rest
          (Utilities|FlowControl|Delay 0.1)
          (Utilities|FlowControl|DoOnce false) ; enters at Reset
        )
        (:then_1
          (Utilities|FlowControl|DoOnce false) ; enters at Reset
        )))
    (:then_1
      ;[0.002964 1 0.03901 1 24] Stop Chasing Player Logic
      (Utilities|FlowControl|DoOnce false) ; enters at Reset
    )
    (:then_2
      ;[0.8745 0.7298 1 1 24] increases/decreases Detection Meter
      (Utilities|FlowControl|DoOnce false) ; enters at Reset
    )
    (:then_3
      ;[0.008364 0.5729 0 1 24] Chasing Player Logic
      (Utilities|FlowControl|DoOnce false) ; enters at Reset
    )))

(event Custom|logic%20move%20in%20path
  (params (Pathing :type BP%20Guard%20Pathing%20Object%20Reference) (PathingNumber :type Integer) (StoptimerAtPath :type Map%20of%20Integers%20to%20Reals) (StopAnimation :type Array%20of%20Anim%20Montage%20Object%20References))
  (bind _spline_path (Variables|/Game/Game/A_Blueprints/NPC/BP_Guard_Pathing.BP_Guard_Pathing_C|GetSpline_path Pathing))
  (bind _stop_point (Variables|AiPath|GetStop%20Point))
  (bind _stopall (Variables|Default|GetStopAll))
  ;[1 0.86 0.3047 0.688 24] Whole Guard Pathing Logic
  ;;[0.5906 0.7083 0.5152 0.844] move in path logic
  (if (Utilities|Map|Contains _stop_point (Variables|AiPath|Getspline%20move%20point))
    (bind _output_get (Variables|AiPath|Setthe%20stop%20animation (.OutItem (Utilities|Array|Random StopAnimation))))
    (Utilities|FlowControl|Delay 0.2)
    (if (not (and (Variables|AiAction|GetIsChasingPlayer) (Variables|aiaction|GetToSoundLocation)))
      (Animation|PlayAnimMontage (Variables|References|GetCharacterRef) _output_get 1.0 "None")
      (Utilities|FlowControl|Delay (.Value (Utilities|Map|Find _stop_point (Variables|AiPath|Getspline%20move%20point))))
      (if (not _stopall)
        (Animation|StopAnimMontage (Variables|References|GetCharacterRef) (Variables|AiPath|Getthe%20stop%20animation))
        (if (not (Math|Boolean|ANDBoolean (Variables|AiAction|GetIsChasingPlayer) (Variables|aiaction|GetToSoundLocation) _stopall))
          (AI|AIMoveTo (Variables|References|GetCharacterRef) (Spline|GetLocationatSplinePoint _spline_path (Variables|AiPath|Getspline%20move%20point) "World") 0 5.0 false :!label _label
            (:OnSuccess
              (if (== (Variables|AiPath|Getspline%20move%20point) (Spline|GetNumberOfSplinePoints _spline_path))
                (Variables|AiPath|Setspline%20move%20point 0)
                (else
                  (Math|Integer|IncrementInt (Variables|AiPath|Getspline%20move%20point)
                    (:%20%20
                      _))))
              (CallFunction|LogicMoveinPath (Variables|References|GetGuardPathingRef) (Variables|AiPath|GetPath%20Number) (Variables|AiPath|GetStop%20Point) (Variables|AiPath|GetStop%20Animation)))))))
    (else
      (Utilities|IsValid _spline_path
        (:Is%20Valid
          (goto _label))))))

(event EventBeginPlay
  ;[0.5487 0.366 1 1 24] Setup
  ;;[1 1 1] setup var
  (Utilities|FlowControl|Sequence
    (:then_0
      (bind _ascharacter (Utilities|Casting|CastToCharacter (Pawn|GetControlledPawn)))
      (bind _output_get (Variables|References|SetCharacterRef _ascharacter))
      (Utilities|IsValid (Actor|GetComponentbyClass _output_get "/Script/Engine.CharacterMovementComponent")
        (:Is%20Valid
          _)
        (:Is%20Not%20Valid
          _))
      (Variables|References|SetGuardMovementCompRef (Actor|GetComponentbyClass _output_get "/Script/Engine.CharacterMovementComponent")))
    (:then_1
      (bind _asbp_player (Utilities|Casting|CastToBP_Player (Game|GetPlayerCharacter 0)))
      (Variables|References|SetPlayerRef _asbp_player))
    (:then_2
      (Utilities|FlowControl|Delay 0.2)
      (bind _aswbp_guard_detection_meter (Utilities|Casting|CastToWBP_Guard_DetectionMeter (UserInterface|GetWidget (Utilities|Array|Get(acopy) (Actor|GetComponentsbyTag (Variables|References|GetCharacterRef) "/Script/UMG.WidgetComponent" "warning")))))
      (bind _output_get_2 (Variables|References|SetDetectionMeterWidget _aswbp_guard_detection_meter))
      (Widget|SetVisibility _output_get_2 "Hidden"))))

(event EventTick
  (params (DeltaSeconds :type Float%20%28single-precision%29))
  ;[0.5487 0.366 1 1 24] Setup
  (Utilities|FlowControl|Sequence
    (:then_0
      (if (Variables|Default|GetStopAll)
        (Variables|Default|SetCurrentTargetDetection 0.0)
        (Widget|SetVisibility (Variables|References|GetDetectionMeterWidget) "Hidden")
        (else
          (Utilities|FlowControl|Sequence
            (:then_0
              (CallFunction|ChasingPlayer)
              (CallFunction|DetectionAction))
            (:then_1
              (CallFunction|LastTimeHasSeenPlayer)
              (CallFunction|CheckBack))))))))

(fn ConstructionScript)

(fn AIPerceptionSight
  (params (actor%20sense :type Actor%20Object%20Reference) (ai%20stimulus :type AI%20Stimulus%20Structure))
  (bind _returnvalue (Class|AIPerceptionSystem|GetSenseClassforStimulus ai%20stimulus))
  (if (== _returnvalue "/Script/AIModule.AISense_Sight")
    (if (.bSuccessfullySensed (Utilities|Struct|BreakAIStimulus ai%20stimulus))
      (if (== (Variables|References|GetPlayerRef) actor%20sense)
        (Variables|AiAction|SetHasSeenPlayer true))
      (else
        (Variables|AiAction|SetHasSeenPlayer false)))
    (else
      (Variables|AiAction|SetHasSeenPlayer false)
      (return))))

(fn ReturntoPathing
  (CallFunction|LogicMoveinPath (Variables|References|GetGuardPathingRef) (Variables|AiPath|GetPath%20Number) (Variables|AiPath|GetStop%20Point) (Variables|AiPath|GetStop%20Animation)))

(fn CalculateDistance
  (return (Transformation|GetDistanceTo (Variables|References|GetCharacterRef) (Variables|References|GetPlayerRef))))

(fn AIPerceptionTouch
  (params (actor%20sense :type Actor%20Object%20Reference) (ai%20stimulus :type AI%20Stimulus%20Structure))
  (bind _returnvalue (Class|AIPerceptionSystem|GetSenseClassforStimulus ai%20stimulus))
  (if (== _returnvalue "/Script/AIModule.AISense_Touch")
    (if (.bSuccessfullySensed (Utilities|Struct|BreakAIStimulus ai%20stimulus))
      (if (== (Variables|References|GetPlayerRef) actor%20sense)
        (Variables|AiAction|SetIsTouchingPlayer true)
        (Variables|Default|SetCurrentTargetDetection 0.95))
      (else
        (Variables|AiAction|SetIsTouchingPlayer false)))
    (else
      (Variables|AiAction|SetIsTouchingPlayer false)
      (return))))

(fn AIPerceptionHearing
  (params (actor%20sense :type Actor%20Object%20Reference) (ai%20stimulus :type AI%20Stimulus%20Structure))
  (bind (_age _expirationage _strength _stimuluslocation _receiverlocation _tag _bsuccessfullysensed) (Utilities|Struct|BreakAIStimulus ai%20stimulus))
  (bind _returnvalue (Class|AIPerceptionSystem|GetSenseClassforStimulus ai%20stimulus))
  (if (== _returnvalue "/Script/AIModule.AISense_Hearing")
    (if _bsuccessfullysensed
      (if (not (Variables|AiAction|GetIsChasingPlayer))
        (if (Actor|ActorHasTag actor%20sense "enemy")
          (CallFunction|MoveAItoSoundLocation _stimuluslocation)
          (Variables|Default|SetCurrentTargetDetection 0.98))))
    (else
      (return))))