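; Placeable tutorial trigger that shows a WBP_Tutorial widget with its configured text when the player enters the start box.
; The widget, created on BeginPlay, fades in with a sound and reverses the fade after a set duration.
; A DoOnce limits overlap triggers unless CanReset re-arms it, while SetTutorial shows the message directly.
; The construction script sizes both boxes and positions the finish box, which has no logic in this graph.
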(event OnComponentBeginOverlap(BoxTutorialStart)
  (params (OverlappedComponent :type Primitive%20Component%20Object%20Reference) (OtherActor :type Actor%20Object%20Reference) (OtherComp :type Primitive%20Component%20Object%20Reference) (OtherBodyIndex :type Integer) (bFromSweep :type Boolean) (SweepResult :type Hit%20Result%20Structure%20%28by%20ref%29))
  (bind _widgetref (Variables|Default|GetWidgetRef))
  (bind _tutorialoverladefadein (Variables|/Game/Game/E_UI/Widgets/WBP_Tutorial.WBP_Tutorial_C|GetTutorialOverladeFadeIn _widgetref))
  (Utilities|FlowControl|DoOnce false
    (:Completed
      (if (== OtherActor (Game|GetPlayerCharacter 0))
        (if (not (Variables|Default|GetIsColliding))
          (Variables|/Game/Game/E_UI/Widgets/WBP_Tutorial.WBP_Tutorial_C|SetTutorialText _widgetref (Variables|Default|GetTutorialText))
          (Audio|PlaySound2D "/Game/Game/D_Audio/SFX/UI/UI_Button_Hover.UI_Button_Hover" 1.0 1.0 0.0 0 0)
          (UserInterface|Viewport|AddtoViewport _widgetref 0)
          (UserInterface|Animation|PlayAnimation _widgetref _tutorialoverladefadein 0.0 1 "Forward" 1.0 false)
          (Utilities|FlowControl|Delay (Variables|Default|GetTutorialDuration))
          (UserInterface|Animation|PlayAnimation _widgetref _tutorialoverladefadein 0.0 1 "Reverse" 1.0 false)
          (Variables|Default|SetTutorialInProgress true)
          (CallFunction|ResetTutorialText))))))

(event Custom|ResetTutorialText
  (bind _widgetref (Variables|Default|GetWidgetRef))
  (bind _tutorialoverladefadein (Variables|/Game/Game/E_UI/Widgets/WBP_Tutorial.WBP_Tutorial_C|GetTutorialOverladeFadeIn _widgetref))
  (if (Variables|Default|GetCanReset)
    (Utilities|FlowControl|DoOnce false) ; enters at Reset
  ))

(event Custom|SetTutorial
  (bind _widgetref (Variables|Default|GetWidgetRef))
  (bind _tutorialoverladefadein (Variables|/Game/Game/E_UI/Widgets/WBP_Tutorial.WBP_Tutorial_C|GetTutorialOverladeFadeIn _widgetref))
  (Variables|/Game/Game/E_UI/Widgets/WBP_Tutorial.WBP_Tutorial_C|SetTutorialText _widgetref (Variables|Default|GetTutorialText))
  (Audio|PlaySound2D "/Game/Game/D_Audio/SFX/UI/UI_Button_Hover.UI_Button_Hover" 1.0 1.0 0.0 0 0)
  (UserInterface|Viewport|AddtoViewport _widgetref 0)
  (UserInterface|Animation|PlayAnimation _widgetref _tutorialoverladefadein 0.0 1 "Forward" 1.0 false)
  (Utilities|FlowControl|Delay (Variables|Default|GetTutorialDuration))
  (UserInterface|Animation|PlayAnimation _widgetref _tutorialoverladefadein 0.0 1 "Reverse" 1.0 false)
  (Variables|Default|SetTutorialInProgress true)
  (CallFunction|ResetTutorialText))

(event EventBeginPlay
  (bind _returnvalue (UserInterface|CreateWidget "/Game/Game/E_UI/Widgets/WBP_Tutorial.WBP_Tutorial_C" 0 (Variables|Default|GetTutorialText)))
  (Variables|Default|SetWidgetRef _returnvalue))

(event Collision|EventActorBeginOverlap
  (params (OtherActor :type Actor%20Object%20Reference)))

(fn ConstructionScript
  (bind _boxtutorialfinish (Variables|Default|GetBoxTutorialFinish))
  (Components|Box|SetBoxExtent (Variables|Default|GetBoxTutorialStart) (Variables|Default|GetBoxTutorialStartSize) true)
  (Components|Box|SetBoxExtent _boxtutorialfinish (Variables|Default|GetBoxTutorialFinishSize) true)
  (Transformation|SetRelativeLocation _boxtutorialfinish (Variables|Default|GetBoxTutorialFinishLocation) false false))